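; Player controller for the spaceship that turns input into stepped movement and quarter-turn rotation.
; The rotate action prints a debug string and adds 90 degrees to control rotation yaw.
; Forward and right axes offset player pawn 0 along its own vectors without sweep, so movement ignores collision.
; A Delay on each axis event throttles movement to periodic steps rather than per-frame motion.
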(event `InputAction|RotationPlayer`
  (params (Key :type "Key Structure"))
  ;[1 1 1] Player Rotate
  (:`Pressed`
    (`KismetSystemLibrary.PrintString` "mmmmmmmmm")
    (`self.SetControlRotation` (`KismetMathLibrary.MakeRotator` (.roll (`self.GetControlRotation`)) (.pitch (`self.GetControlRotation`)) (+ (.yaw (`self.GetControlRotation`)) 90.0)))))

(event `InputAxis|moveForward`
  (params (AxisValue :type "Float (single-precision)"))
  ;[1 1 1] Player Move Forward
  (`KismetSystemLibrary.Delay` 0.1)
  (`self.K2_AddActorWorldOffset` (`GameplayStatics.GetPlayerPawn` 0) (* (`self.GetActorForwardVector` (`GameplayStatics.GetPlayerPawn` 0)) (* AxisValue 50.0)) false false))

(event `InputAxis|MoveRight`
  (params (AxisValue :type "Float (single-precision)"))
  ;[1 1 1] Player Move Right
  (`KismetSystemLibrary.Delay` 0.1)
  (`self.K2_AddActorWorldOffset` (`GameplayStatics.GetPlayerPawn` 0) (* (`self.GetActorRightVector` (`GameplayStatics.GetPlayerPawn` 0)) (* AxisValue 50.0)) false false))

(fn `UserConstructionScript`)